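; Player controller for a MapleStory-style game that handles character selection, spawning and possession of the chosen character.
; On BeginPlay, a client event creates the character select widget and adds it to the viewport.
; Selections pass through a server event to the game mode as a spawn request, using interface-style reference getters.
; SpawnPlayers spawns the given class at the supplied transform and possesses it.
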(event `self.ReceiveBeginPlay`
  (`/Game/Blueprints/Interface/Int_PLayerController.InitializeWidgets`))

(event `/Game/Blueprints/Interface/Int_PLayerController.InitializeWidgets`
  (`self.Client_InitializeWidgets`))

(event `Client_InitializeWidgets`
  (bind _returnvalue (`|CreateWidget` "/Game/UI/WB_CharacterSelect.WB_CharacterSelect_C"))
  (bind _output_get (set `self.CharacterSelection` _returnvalue))
  (`UserWidget.AddToViewport` _output_get 0))

(event `/Game/Blueprints/Interface/Int_PLayerController.SelectCharacter`
  (params (Player :type "Actor Class Reference") (SpawnLocation :type "Vector Structure"))
  (`self.SRV_SelectCharacter` Player SpawnLocation))

(event `SRV_SelectCharacter`
  (params (Player :type "Actor Class Reference") (SpawnLocation :type "Vector Structure"))
  (bind _gamemode (message `/Game/Blueprints/Interface/Int_GameMode.GetGameModeRef` (`GameplayStatics.GetGameMode`)))
  (message `/Game/Blueprints/Interface/Int_GameMode.RequestSpawnPlayer` _gamemode self Player SpawnLocation))

(event `/Game/Blueprints/Interface/Int_PLayerController.SpawnPlayers`
  (params (Player :type "Actor Class Reference") (SpawnTransform :type "Transform Structure"))
  (bind _returnvalue (`|SpawnActorFromClass` Player SpawnTransform "Undefined" "MultiplyWithRoot" null null))
  (bind _player (message `/Game/Blueprints/Interface/Int_PlayerBase.GetPlayerRef` _returnvalue))
  (`self.Possess` _player))

(fn `GetPlayerControllerRef`
  (returns (PlayerController :type "/Game/Blueprints/PC_MapleStory Object Reference"))
  (return self))

(fn `UserConstructionScript`)