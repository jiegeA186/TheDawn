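; Base Paper2D enemy character with replicated animation states and data from an AnimalInfo struct.
; Movement state changes go through SRV_SetMovementState, and rep-notifies on MovementState and IsMoving swap the sprite's idle, move or hit flipbook.
; Any damage sets the Hit state, disables movement and writes Health as clamped Damage minus Health, an inverted subtraction.
; GetEnemyRef returns self; the only IsMoving write is unreachable.
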(event `/Game/Blueprints/Interface/Int_EnemyBase.SetMovementState`
  (params (MovementSStates :type "/Game/Blueprints/Enums/E_MovementStates Enum" :default "NewEnumerator0"))
  (`self.SRV_SetMovementState` MovementSStates))

(event `SRV_SetMovementState`
  (params (Movementstate :type "/Game/Blueprints/Enums/E_MovementStates Enum" :default "NewEnumerator0"))
  (set `self.MovementState` Movementstate))

(event `self.ReceiveAnyDamage`
  (params (Damage :type "Float (single-precision)") (DamageType :type "DamageType Object Reference") (InstigatedBy :type "Controller Object Reference") (DamageCauser :type "Actor Object Reference"))
  (bind _animalinfo (`self.AnimalInfo`))
  (bind _health (break `/Game/Blueprints/Structure/ST_AnimalInfo` _animalinfo))
  (`/Game/Blueprints/Interface/Int_EnemyBase.SetMovementState` "NewEnumerator7")
  (`CharacterMovementComponent.SetMovementMode` (`self.CharacterMovement`) "MOVE_None" 0)
  (bind _structout (setmembers `/Game/Blueprints/Structure/ST_AnimalInfo` :`StructRef` _animalinfo :`Health` (`KismetMathLibrary.FClamp` (- Damage _health) 0.0 _health)))
  (set `self.AnimalInfo` _structout))

(fn `GetEnemyRef`
  (returns (Enemy :type "/Game/Blueprints/Enemy/BP_EnemyBase Object Reference"))
  (return self))

(fn `OnRep_IsMoving`
  (bind _sprite (`self.Sprite`))
  (bind (_health _idleanimation _moveanimation) (break `/Game/Blueprints/Structure/ST_AnimalInfo` (`self.AnimalInfo`)))
  (if (not (`self.IsMoving`))
    (`PaperFlipbookComponent.SetFlipbook` _sprite _idleanimation)
    (else
      (`PaperFlipbookComponent.SetFlipbook` _sprite _moveanimation))))

(fn `OnRep_MovementState`
  (bind _sprite (`self.Sprite`))
  (bind (_health _idleanimation _moveanimation _hitanimation) (break `/Game/Blueprints/Structure/ST_AnimalInfo` (`self.AnimalInfo`)))
  (switch `/Game/Blueprints/Enums/E_MovementStates` (`self.MovementState`)
    (:`NewEnumerator0`
      (`PaperFlipbookComponent.SetFlipbook` _sprite _idleanimation))
    (:`NewEnumerator1`
      (`PaperFlipbookComponent.SetFlipbook` _sprite _moveanimation))
    (:`NewEnumerator7`
      (`PaperFlipbookComponent.SetFlipbook` _sprite _hitanimation))))

(fn `UserConstructionScript`
  (`parent.UserConstructionScript`))